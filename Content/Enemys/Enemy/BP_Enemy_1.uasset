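; Enemy tank that chases the player, shoots at them and drops an experience crystal when destroyed.
; Every Tick turns the turret mesh's yaw toward the player at constant speed, advances the fire timer and re-issues an AI MoveTo.
; Reaching the player's radius calls Disparar, which spawns a bullet and shot sound at the turret socket, limited by FireRate.
; Damage lowers Health and activates sparks; Tick handles death once Health runs out.
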(event Custom|Follow_Player
  (AI|AIMoveTo self "0, 0, 0" (Game|GetPlayerCharacter 0) 5.5e+02 false
    (:OnSuccess
      (CallFunction|Disparar))))

(event EventBeginPlay
  (Variables|Default|SetJugador (Game|GetPlayerCharacter 0)))

(event Collision|EventActorBeginOverlap
  (params (OtherActor :type Actor%20Object%20Reference)))

(event EventTick
  (params (DeltaSeconds :type Float%20%28single-precision%29))
  (Variables|Default|SetDeltaS DeltaSeconds)
  (CallFunction|Apuntar)
  (Variables|Default|SetFireRateDelta (+ (Variables|Default|GetFireRateDelta) (Utilities|Time|GetWorldDeltaSeconds)))
  (CallFunction|FollowPlayer)
  (if (<= (Variables|Default|GetHealth) 0)
    (Game|SpawnActorfromClass "/Game/Characters/Obejtos/BP_CristalExperiencia.BP_CristalExperiencia_C" (Math|Transform|MakeTransform (Transformation|GetActorLocation) (Math|Rotator|MakeRotator 0.0 0.0 0.0) "1.000000,1.000000,1.000000") "Undefined" "MultiplyWithRoot" 0 0)
    (Actor|DestroyActor)))

(event Game|Damage|EventAnyDamage
  (params (Damage :type Float%20%28single-precision%29) (DamageType :type Damage%20Type%20Object%20Reference) (InstigatedBy :type Controller%20Object%20Reference) (DamageCauser :type Actor%20Object%20Reference))
  (Variables|Default|SetHealth (- (Variables|Default|GetHealth) Damage))
  (Components|Activation|Activate (Variables|Default|GetP_Sparks_E) false))

(fn ConstructionScript)

(fn Apuntar
  (bind _tanque_polysurface22 (Variables|Default|GetTanque_polySurface22))
  (Transformation|SetWorldRotation (Variables|Default|GetTanque_polySurface22) (Math|Rotator|MakeRotator 0.0 0.0 (.yaw (Class|KismetMathLibrary|RInterptoConstant (Math|Rotator|MakeRotator 0.0 0.0 (.yaw (Transformation|GetWorldRotation _tanque_polysurface22))) (Math|Rotator|MakeRotator 0.0 0.0 (- (.yaw (Math|Rotator|FindLookatRotation (Transformation|GetWorldLocation _tanque_polysurface22) (Transformation|GetActorLocation (Variables|Default|GetJugador)))) 9e+01)) (Variables|Default|GetDeltaS) 1e+02))) false false))

(fn Disparar
  (bind _nombresoket (Variables|Default|GetNombreSoket))
  (bind _tanque_polysurface22 (Variables|Default|GetTanque_polySurface22))
  (bind _returnvalue (Transformation|GetSocketLocation _tanque_polysurface22 _nombresoket))
  (if (>= (Variables|Default|GetFireRateDelta) (Variables|Default|GetFireRate))
    (Variables|Default|SetFireRateDelta 0.0)
    (Game|SpawnActorfromClass "/Game/Armas/BP_BalaEnemigo.BP_BalaEnemigo_C" (Math|Transform|MakeTransform _returnvalue (Math|Rotator|MakeRotator 0.0 0.0 (.yaw (Transformation|GetSocketRotation _tanque_polysurface22 _nombresoket))) "1.000000,1.000000,1.000000") "Undefined" "MultiplyWithRoot" 0 0)
    (Audio|SpawnSoundatLocation "/Game/Sonido/M14-Shot-QuickSounds-recortado.M14-Shot-QuickSounds-recortado" _returnvalue "0, 0, 0" 1.0 1.0 0.0 0 0)))