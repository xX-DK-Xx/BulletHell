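; Kamikaze tank enemy that chases the player and explodes on reaching them, dealing damage with an effect and sound.
; Each tick it turns its mesh toward the player and calls the AI MoveTo chase.
; At zero health it drops an experience crystal or, less often, shotgun or explosive ammo.
; After death or explosion it is recycled, teleporting along the mesh's right vector and resetting health instead of being destroyed.
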(event Custom|Follow_Player
  (AI|AIMoveTo self "0, 0, 0" (Game|GetPlayerCharacter 0) 1.5e+02 false
    (:OnSuccess
      (CallFunction|Implosion)
      (Transformation|SetActorLocation (+ (Transformation|GetActorLocation) (* (Math|Vector|GetRightVector (Variables|Default|GetTanque_polySurface22)) "400.000000,400.000000,0.000000")) false true)
      (Variables|Default|SetHealth 40))))

(event EventBeginPlay
  (Variables|Default|SetJugador (Game|GetPlayerCharacter 0)))

(event Collision|EventActorBeginOverlap
  (params (OtherActor :type Actor%20Object%20Reference)))

(event EventTick
  (params (DeltaSeconds :type Float%20%28single-precision%29))
  (bind _returnvalue (Transformation|GetActorLocation))
  (bind _returnvalue_2 (Math|Random|RandomFloat))
  (Variables|Default|SetDeltaS DeltaSeconds)
  (CallFunction|Apuntar)
  (Variables|Default|SetFireRateDelta (+ (Variables|Default|GetFireRateDelta) (Utilities|Time|GetWorldDeltaSeconds)))
  (CallFunction|FollowPlayer)
  (if (<= (Variables|Default|GetHealth) 0)
    (if (> _returnvalue_2 0.3)
      (Game|SpawnActorfromClass "/Game/Characters/Obejtos/BP_CristalExperiencia.BP_CristalExperiencia_C" (Math|Transform|MakeTransform _returnvalue "0, 0, 0" "1.000000,1.000000,1.000000") "Undefined" "MultiplyWithRoot" 0 0)
      (elif (> _returnvalue_2 0.5)
        (Game|SpawnActorfromClass "/Game/Characters/Obejtos/BP_MunicionEscopeta.BP_MunicionEscopeta_C" (Math|Transform|MakeTransform _returnvalue "0, 0, 0" "1.000000,1.000000,1.000000") "Undefined" "MultiplyWithRoot" 0 0)
        (else
          (Game|SpawnActorfromClass "/Game/Characters/Obejtos/BP_MunicionExplosiva.BP_MunicionExplosiva_C" (Math|Transform|MakeTransform _returnvalue "0, 0, 0" "1.000000,1.000000,1.000000") "Undefined" "MultiplyWithRoot" 0 0))))
    (Transformation|SetActorLocation (+ (Transformation|GetActorLocation) (* (Math|Vector|GetRightVector (Variables|Default|GetTanque_polySurface22)) "400.000000,400.000000,0.000000")) false true)
    (Variables|Default|SetHealth 40)))

(event Game|Damage|EventAnyDamage
  (params (Damage :type Float%20%28single-precision%29) (DamageType :type Damage%20Type%20Object%20Reference) (InstigatedBy :type Controller%20Object%20Reference) (DamageCauser :type Actor%20Object%20Reference))
  (Variables|Default|SetHealth (- (Variables|Default|GetHealth) Damage)))

(fn ConstructionScript)

(fn Apuntar
  (bind _tanque_polysurface22 (Variables|Default|GetTanque_polySurface22))
  (Transformation|SetWorldRotation (Variables|Default|GetTanque_polySurface22) (Math|Rotator|MakeRotator 0.0 0.0 (.yaw (Class|KismetMathLibrary|RInterptoConstant (Math|Rotator|MakeRotator 0.0 0.0 (.yaw (Transformation|GetWorldRotation _tanque_polysurface22))) (Math|Rotator|MakeRotator 0.0 0.0 (- (.yaw (Math|Rotator|FindLookatRotation (Transformation|GetWorldLocation _tanque_polysurface22) (Transformation|GetActorLocation (Variables|Default|GetJugador)))) 9e+01)) (Variables|Default|GetDeltaS) 1e+02))) false false))

(fn Implosion
  (bind _returnvalue (Transformation|GetActorLocation))
  (Game|Damage|ApplyDamage (Game|GetPlayerCharacter 0) 3e+01 0 0)
  (Effects|SpawnEmitteratLocation "/Game/Realistic_Starter_VFX_Pack_Vol2/Particles/Explosion/P_Explosion_Big_A.P_Explosion_Big_A" _returnvalue "0, 0, 0" "2.000000,2.000000,2.000000")
  (Audio|SpawnSoundatLocation "/Game/Sonido/medium-explosion-40472.medium-explosion-40472" _returnvalue "0, 0, 0" 1.0 1.0 0.0 0 0))