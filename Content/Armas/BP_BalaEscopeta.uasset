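; BP_BalaEscopeta is the shotgun bullet projectile that damages what it hits.
; On BeginPlay it caches the player's BP_TopDownCharacter to read its damage multiplier.
; On overlap it ignores the player character and other shotgun bullets; anything else takes the bullet's damage scaled by that multiplier.
; It then plays an explosion sound at its location and destroys itself.
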(event EventBeginPlay
  (bind _asbp_top_down_character (Utilities|Casting|CastToBP_TopDownCharacter (Game|Player|GetPlayerPawn 0)))
  (Variables|Default|SetReferenciaPersonaje _asbp_top_down_character))

(event Collision|EventActorBeginOverlap
  (params (OtherActor :type Actor%20Object%20Reference))
  (Utilities|Casting|CastToBP_TopDownCharacter OtherActor
    (:CastFailed
      (Utilities|Casting|CastToBP_BalaEscopeta OtherActor
        (:CastFailed
          (Game|Damage|ApplyDamage OtherActor (* (Variables|Default|GetDMG) (Variables|/Game/TopDown/Blueprints/BP_TopDownCharacter.BP_TopDownCharacter_C|GetMultiploDMG (Variables|Default|GetReferenciaPersonaje))) 0 0)
          (Audio|SpawnSoundatLocation "/Game/Sonido/medium-explosion-40472.medium-explosion-40472" (Transformation|GetActorLocation) "0, 0, 0" 1.0 1.0 0.0 0 0)
          (Actor|DestroyActor))))))

(event EventTick
  (params (DeltaSeconds :type Float%20%28single-precision%29)))

(fn ConstructionScript)