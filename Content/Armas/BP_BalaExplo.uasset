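; BP_BalaExplo is an explosive bullet that detonates when it hits anything other than the top-down player character.
; On BeginPlay it caches the player's BP_TopDownCharacter to read that character's damage multiplier.
; On impact it spawns a large explosion effect and sound, applies radial damage scaled by that multiplier while ignoring the player, then destroys itself.
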(event EventBeginPlay
  (bind _asbp_top_down_character (Utilities|Casting|CastToBP_TopDownCharacter (Game|Player|GetPlayerPawn 0)))
  (Variables|Default|SetReferenciaPersonaje _asbp_top_down_character))

(event EventTick
  (params (DeltaSeconds :type Float%20%28single-precision%29)))

(event Collision|EventHit
  (params (MyComp :type Primitive%20Component%20Object%20Reference) (Other :type Actor%20Object%20Reference) (OtherComp :type Primitive%20Component%20Object%20Reference) (bSelfMoved :type Boolean) (HitLocation :type Vector :default "0, 0, 0") (HitNormal :type Vector :default "0, 0, 0") (NormalImpulse :type Vector :default "0, 0, 0") (Hit :type Hit%20Result%20Structure%20%28by%20ref%29))
  (Utilities|Casting|CastToBP_TopDownCharacter Other
    (:CastFailed
      (Effects|SpawnEmitteratLocation "/Game/Realistic_Starter_VFX_Pack_Vol2/Particles/Explosion/P_Explosion_Big_A.P_Explosion_Big_A" HitLocation)
      (Game|Damage|ApplyRadialDamage (* (Variables|Default|GetDMG) (Variables|/Game/TopDown/Blueprints/BP_TopDownCharacter.BP_TopDownCharacter_C|GetMultiploDMG (Variables|Default|GetReferenciaPersonaje))) HitLocation 1e+02 0 (Utilities|Array|MakeArray (Variables|Default|GetReferenciaPersonaje)) 0 0 false "ECC_Visibility")
      (Audio|SpawnSoundatLocation "/Game/Sonido/medium-explosion-40472.medium-explosion-40472" (Transformation|GetActorLocation) "0, 0, 0" 1.0 1.0 0.0 0 0)
      (Actor|DestroyActor))))

(fn ConstructionScript)